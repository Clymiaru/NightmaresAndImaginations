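; Toy chest actor that shows an interaction prompt while something overlaps its InteractRange.
; BeginPlay creates the hidden prompt widget, and the range's overlap events toggle its visibility and an overlap flag.
; The GetItem input sets an interacting flag, which Tick reads during overlap to choose UI-only input with a cursor or game-only input.
; The interacting flag is never cleared by connected logic, and debug prints remain throughout.
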(event `self.ReceiveTick`
  (params (DeltaSeconds :type "Float (single-precision)"))
  (bind _returnvalue (`GameplayStatics.GetPlayerController` 0))
  (if (`self.isOverlapping`)
    (if (`self.isInteracting`)
      (`KismetSystemLibrary.PrintString` "Update")
      (set `PlayerController.bShowMouseCursor` true _returnvalue)
      (`WidgetBlueprintLibrary.SetInputMode_UIOnlyEx` _returnvalue null)
      (else
        (set `PlayerController.bShowMouseCursor` false _returnvalue)
        (`WidgetBlueprintLibrary.SetInputMode_GameOnly` _returnvalue)))))

(event `self.ReceiveBeginPlay`
  (bind _returnvalue (`|CreateWidget` "/Game/Widgets/InteractPrompt_HUD.InteractPrompt_HUD_C"))
  (bind _output_get (set `self.InteractPrompt_HUD` _returnvalue))
  (`UserWidget.AddToViewport` _output_get 0)
  (`Widget.SetVisibility` (`self.InteractPrompt_HUD`) "Hidden"))

(event `InputAction|GetItem`
  (params (Key :type "Key Structure"))
  (:`Pressed`
    (set `self.isInteracting` true)
    (`KismetSystemLibrary.PrintString` "Press F")))

(event `self.InteractRange.OnComponentBeginOverlap`
  (params (OverlappedComponent :type "PrimitiveComponent Object Reference") (OtherActor :type "Actor Object Reference") (OtherComp :type "PrimitiveComponent Object Reference") (OtherBodyIndex :type Integer) (bFromSweep :type Boolean) (SweepResult :type "HitResult Structure (by ref)"))
  (set `self.isOverlapping` true)
  (`KismetSystemLibrary.PrintString` "Enter interaction")
  (`Widget.SetVisibility` (`self.InteractPrompt_HUD`) "Visible"))

(event `self.InteractRange.OnComponentEndOverlap`
  (params (OverlappedComponent :type "PrimitiveComponent Object Reference") (OtherActor :type "Actor Object Reference") (OtherComp :type "PrimitiveComponent Object Reference") (OtherBodyIndex :type Integer))
  (set `self.isOverlapping` false)
  (`KismetSystemLibrary.PrintString` "Exit interaction")
  (`Widget.SetVisibility` (`self.InteractPrompt_HUD`) "Hidden"))

(fn `UserConstructionScript`)