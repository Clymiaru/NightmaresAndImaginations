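; VictoryPortal is an actor that declares the game won once no SimpleAI enemies remain in the level.
; BeginPlay caches the VictoryUI widget from MainPlayerController_BP.
; Tick runs through a three-second Delay, polling for SimpleAI actors; finding none shows the cursor, switches to UI-only input and sets IsGameWon.
; A later delayed pass makes the victory widget visible, with no overlap logic involved.
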(event `self.ReceiveBeginPlay`
  (bind _asmain_player_controller_bp (cast `/Game/Blueprints/MainPlayerController_BP` (`GameplayStatics.GetPlayerController` 0)))
  (set `self.Victory_user_interface` (`/Game/Blueprints/MainPlayerController_BP.VictoryUI` _asmain_player_controller_bp)))

(event `self.ReceiveTick`
  (params (DeltaSeconds :type "Float (single-precision)"))
  ;[1 1 1] Search Alive Enemies
  (`KismetSystemLibrary.Delay` 3.0)
  (if (`self.isGameWon`)
    (`Widget.SetVisibility` (`self.Victory_user_interface`) "Visible")
    (else
      (bind _outactors (`GameplayStatics.GetAllActorsOfClass` "/Game/ThirdPersonBP/Blueprints/SimpleAI.SimpleAI_C"))
      (set `self.FindEnemies` true)
      (if (== (`KismetArrayLibrary.Array_Length` _outactors) 0)
        (set `PlayerController.bShowMouseCursor` true (`GameplayStatics.GetPlayerController` 0))
        (`WidgetBlueprintLibrary.SetInputMode_UIOnlyEx` (`GameplayStatics.GetPlayerController` 0) null)
        (set `self.isGameWon` true)))))

(fn `UserConstructionScript`)