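; MainPlayerController_BP is the player controller that sets up the player UI and syncs some state with the main character.
; BeginPlay creates the HUD and inventory display widgets and adds them to the viewport.
; Every Tick, it copies its Attacking flag into the character's Attack1h for attack animation.
; Its AnyDamage event disables the character's capsule collision once current HP reaches zero or below.
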(event `self.ReceiveBeginPlay`
  ;[1 1 1] UI
  (bind _returnvalue (`|CreateWidget` "/Game/ThirdPersonBP/Blueprints/Player_Hud.Player_HUD_C" self))
  (`UserWidget.AddToViewport` _returnvalue 0)
  (bind _returnvalue_2 (`|CreateWidget` "/Game/Widgets/InventoryDIsplay.InventoryDIsplay_C" self))
  (`UserWidget.AddToViewport` _returnvalue_2 0))

(event `self.ReceiveTick`
  (params (DeltaSeconds :type "Float (single-precision)"))
  ;[1 1 1] attack animation purposes
  (bind _asmain_character_bp (cast `/Game/ThirdPersonBP/Blueprints/MainCharacter_BP` (`GameplayStatics.GetPlayerCharacter` 0)))
  (set `/Game/ThirdPersonBP/Blueprints/MainCharacter_BP.Attack1h` (`self.attacking`) _asmain_character_bp))

(event `self.ReceiveAnyDamage`
  (params (Damage :type "Float (single-precision)") (DamageType :type "DamageType Object Reference") (InstigatedBy :type "Controller Object Reference") (DamageCauser :type "Actor Object Reference"))
  ;[1 1 1] Take Damage
  (bind _asmain_character_bp (cast `/Game/ThirdPersonBP/Blueprints/MainCharacter_BP` (`GameplayStatics.GetPlayerCharacter` 0)))
  (if (<= (`CharacterStatsComponent.currHp` (`/Game/ThirdPersonBP/Blueprints/MainCharacter_BP.CharacterStats` _asmain_character_bp)) 0.0)
    (`PrimitiveComponent.SetCollisionEnabled` (`Character.CapsuleComponent` _asmain_character_bp) "NoCollision")))

(fn `UserConstructionScript`)