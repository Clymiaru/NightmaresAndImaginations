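; RockBlock_BP is a destructible rock that becomes breakable once no SimpleAI enemies remain in the level.
; Tick watches the player's Attack1h flag and uses a FindEnemies latch to count SimpleAI actors once per attack.
; When none are found, collision moves from the Collider to the Destructible, which starts with collision off.
; On fracture, it plays a rockslide sound at world origin and destroys itself after a short delay.
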(event `self.ReceiveBeginPlay`
  (bind _asmain_character_bp (cast `/Game/ThirdPersonBP/Blueprints/MainCharacter_BP` (`GameplayStatics.GetPlayerCharacter` 0)))
  (set `self.MainCharacter` _asmain_character_bp)
  (`PrimitiveComponent.SetCollisionEnabled` (`self.Destructible`) "NoCollision"))

(event `self.ReceiveTick`
  (params (DeltaSeconds :type "Float (single-precision)"))
  (bind _attack1h (`/Game/ThirdPersonBP/Blueprints/MainCharacter_BP.Attack1h` (`self.MainCharacter`)))
  ;[1 1 1] Search Alive Enemies
  (if _attack1h
    (if _attack1h
      (if (not (`self.FindEnemies`))
        (bind _outactors (`GameplayStatics.GetAllActorsOfClass` "/Game/ThirdPersonBP/Blueprints/SimpleAI.SimpleAI_C"))
        (set `self.FindEnemies` true)
        ;[1 1 1] Make rock interactable
        (if (== (`KismetArrayLibrary.Array_Length` _outactors) 0)
          (`PrimitiveComponent.SetCollisionEnabled` (`self.Destructible`) "QueryAndPhysics")
          (`PrimitiveComponent.SetCollisionEnabled` (`self.Collider`) "NoCollision"))))
    (else
      (set `self.FindEnemies` false))))

(event `self.Destructible.OnComponentFracture`
  (params (HitPoint :type "Vector Structure (by ref)") (HitDirection :type "Vector Structure (by ref)"))
  ;[1 1 1] On Fracture Actor
  (`GameplayStatics.PlaySoundAtLocation` "/Game/Audio/rockslide_Cue.rockslide_Cue" (0.0 0.0 0.0) (struct) 1.0 1.0 0.0 null null null)
  (`KismetSystemLibrary.Delay` 1.0)
  (`self.K2_DestroyActor`))

(fn `UserConstructionScript`)